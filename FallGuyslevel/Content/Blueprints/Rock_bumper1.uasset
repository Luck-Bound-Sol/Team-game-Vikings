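; Rock bumper actor that bounces the player character away when it enters the bumper's overlap area.
; On overlap with BP_ThirdPersonCharacter2, it nudges the character upward with a swept move.
; It then applies a velocity-change impulse to the character's movement, opposing the combined bumper and player velocity in X and Y, scaled by Bunecyness, with Z zeroed.
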(event `self.ReceiveActorBeginOverlap`
  (params (OtherActor :type "Actor Object Reference"))
  ;[1 1 1] Bounce Player by aplying an inpuse opastit there movement
  ;;[1 1 1] See if it is a player that enterned to trigger zone
  (bind _asbp_third_person_character_2 (cast `/Game/ThirdPerson/Blueprints/BP_ThirdPersonCharacter2` OtherActor))
  (`self.K2_SetActorLocation` _asbp_third_person_character_2 (+ (`self.K2_GetActorLocation` _asbp_third_person_character_2) (0.0 0.0 50.0)) true false)
  ;;[1 1 1] Added the impuse to the player movement
  (`CharacterMovementComponent.AddImpulse` (`Character.CharacterMovement` _asbp_third_person_character_2) (* (+ (`self.GetVelocity`) (`self.GetVelocity` _asbp_third_person_character_2)) (* (`self.Bunecyness`) (-1.0 -1.0 0.0))) true))

(event `self.ReceiveBeginPlay`)

(fn `UserConstructionScript`)