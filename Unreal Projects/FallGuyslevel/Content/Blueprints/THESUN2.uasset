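; THESUN2 is a moving hazard actor that destroys the player's BP_ThirdPersonCharacter2 on overlap.
; Its construction script builds two relative InterpToMovement control points from Location1 and Location2 and applies the Duration variable, so the path and timing are set per instance.
; On ActorBeginOverlap it casts the other actor to the character class and destroys it, ignoring anything else.
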(event `self.ReceiveActorBeginOverlap`
  (params (OtherActor :type "Actor Object Reference"))
  (bind _asbp_third_person_character_2 (cast `/Game/ThirdPerson/Blueprints/BP_ThirdPersonCharacter2` OtherActor))
  (`self.K2_DestroyActor` _asbp_third_person_character_2))

(fn `UserConstructionScript`
  (bind _interptomovement (`self.InterpToMovement`))
  (set `InterpToMovementComponent.ControlPoints` (`|MakeArray` (make `InterpControlPoint` (`self.Location1`)) (make `InterpControlPoint` (`self.Location2`))) _interptomovement)
  (set `InterpToMovementComponent.Duration` (`self.Duration`) _interptomovement))