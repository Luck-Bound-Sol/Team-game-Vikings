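; SpinePathreverse is an actor Blueprint set up for moving along a spline, apparently in reverse, but its movement logic is unfinished.
; BeginPlay looks up a SpinePath actor without storing it.
; MoveObject feeds TimeToComplete directly into MoveObjectT's play rate and plays Timeline_0.
; The spline transform update is disconnected, its SelectFloat fixes distance at -1, and the length-based Lerp is unused, so the actor never moves.
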(event `self.ReceiveBeginPlay`
  (`GameplayStatics.GetActorOfClass` "/Game/Blueprints/SpinePath.SpinePath_C"))

(event `Move Object`
  (`TimelineComponent.SetPlayRate` (`self.Move Object T`) (`KismetMathLibrary.SelectFloat` 0.0 (`self.Time to complete`)))
  (bind (_direction _move_track) (`Timeline|Timeline_0`)))

(fn `UserConstructionScript`)