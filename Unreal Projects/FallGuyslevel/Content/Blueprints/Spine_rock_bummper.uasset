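; Rock bumper actor, judging by its name, that positions itself on the spline of a SpinePath actor found in the level.
; BeginPlay starts the MoveObjectT timeline, using TimeToComplete directly as its play rate.
; The MoveTrack value is mapped to spline distance to set location and rotation.
; The transform is set once in BeginPlay, with no timeline update wired, and rotation is sampled in local space, location in world space.
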(event `self.ReceiveBeginPlay`
  (bind _spline (`/Game/Blueprints/SpinePath.Spline` (`self.NewVar_0`)))
  (bind _returnvalue (`GameplayStatics.GetActorOfClass` "/Game/Blueprints/SpinePath.SpinePath_C"))
  (set `self.NewVar_0` _returnvalue)
  (`self.Move Object`)
  (bind _returnvalue_2 (`KismetMathLibrary.Lerp` 0.0 (`SplineComponent.GetSplineLength` (`/Game/Blueprints/SpinePath.Spline` (`self.NewVar_0`))) (stale `Move Object` _move_track)))
  (`self.K2_SetActorTransform` (`KismetMathLibrary.MakeTransform` (`SplineComponent.GetLocationAtDistanceAlongSpline` _spline _returnvalue_2 "World") (`SplineComponent.GetRotationAtDistanceAlongSpline` _spline _returnvalue_2 "Local"))))

(event `Move Object`
  (`TimelineComponent.SetPlayRate` (`self.Move Object T`) (`KismetMathLibrary.SelectFloat` 1.0 (`self.Time to complete`)))
  (bind (_direction _move_track) (`Timeline|Move Object T` :!via `PlayFromStart`)))

(fn `UserConstructionScript`)